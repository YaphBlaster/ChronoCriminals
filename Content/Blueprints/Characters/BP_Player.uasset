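; BP_Player is a first-person-style player character with two switchable abilities, Time Shift and Time Slow, shown on a HUD widget.
; Time Shift line-traces from the camera and messages actors implementing BP_Shift.
; Time Slow briefly lowers global time dilation, inversely scaling its own to keep normal speed.
; Interact spawns BP_Bullet; physics-handle pickup, drop, launch and outline logic remain but are disconnected.
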(event `self.ReceiveBeginPlay`
  (bind _returnvalue (`|CreateWidget` "/Game/Blueprints/Widgets/HUD.HUD_C"))
  (bind _output_get (set `self.WidgetReference` _returnvalue))
  (`UserWidget.AddToPlayerScreen` _output_get 0)
  (set `/Game/Blueprints/Widgets/HUD.Ability` (`|GetEnumeratorNameAsString` (`self.Abilities`)) (`self.WidgetReference`)))

(event `InputAxis|MoveForward`
  (params (AxisValue :type "Float (single-precision)"))
  (bind (_returnvalue_roll _returnvalue_pitch _returnvalue_yaw) (`KismetMathLibrary.BreakRotator` (`self.GetControlRotation`)))
  ;[0 0 0] MoveCharacter[DefaultCharacterNodes]
  (`self.AddMovementInput` (`KismetMathLibrary.GetForwardVector` (`KismetMathLibrary.MakeRotator` 0.0 0.0 _returnvalue_yaw)) AxisValue))

(event `InputAxis|MoveRight`
  (params (AxisValue :type "Float (single-precision)"))
  (bind (_returnvalue_roll _returnvalue_pitch _returnvalue_yaw) (`KismetMathLibrary.BreakRotator` (`self.GetControlRotation`)))
  ;[0 0 0] MoveCharacter[DefaultCharacterNodes]
  (`self.AddMovementInput` (`KismetMathLibrary.GetRightVector` (`KismetMathLibrary.MakeRotator` 0.0 0.0 _returnvalue_yaw)) AxisValue))

(event `InputAction|Jump`
  (params (Key :type "Key Structure"))
  ;[0 0 0] Jump[DefaultCharacterNodes]
  (:`Pressed`
    (`self.Jump`))
  (:`Released`
    (`self.StopJumping`)))

(event `InputAxis|Turn`
  (params (AxisValue :type "Float (single-precision)"))
  ;[0 0 0] MouseRotation[DefaultCharacterNodes]
  (`self.AddControllerYawInput` AxisValue))

(event `InputAxis|LookUp`
  (params (AxisValue :type "Float (single-precision)"))
  ;[0 0 0] MouseRotation[DefaultCharacterNodes]
  (`self.AddControllerPitchInput` AxisValue))

(event `InputAction|ChangeAbility`
  (params (Key :type "Key Structure"))
  (:`Pressed`
    (switch `/Game/Blueprints/BP_Abilities` (`self.Abilities`)
      (:`NewEnumerator0`
        (set `self.Abilities` "NewEnumerator1"))
      (:`NewEnumerator1`
        (set `self.Abilities` "NewEnumerator0")))
    (set `/Game/Blueprints/Widgets/HUD.Ability` (`|GetEnumeratorNameAsString` (`self.Abilities`)) (`self.WidgetReference`))))

(event `InputAction|UseAbility`
  (params (Key :type "Key Structure"))
  (:`Pressed`
    (switch `/Game/Blueprints/BP_Abilities` (`self.Abilities`)
      (:`NewEnumerator0`
        (`self.ShiftObject`))
      (:`NewEnumerator1`
        (`self.SlowTime`)))))

(event `ShiftObject`
  (bind _camera (`self.Camera`))
  (bind _returnvalue (`SceneComponent.K2_GetComponentLocation` _camera))
  ;[1 1 1] Shift Object
  (bind _outhit (`KismetSystemLibrary.LineTraceSingle` _returnvalue (+ _returnvalue (* (`SceneComponent.GetForwardVector` _camera) 1000.0)) "TraceTypeQuery1"))
  (bind (_bblockinghit _binitialoverlap _time _distance _location _impactpoint _normal _impactnormal _physmat _hitactor) (`GameplayStatics.BreakHitResult` _outhit))
  (if (`KismetSystemLibrary.DoesImplementInterface` _hitactor "/Game/Blueprints/Interfaces/BP_Shift.BP_Shift_C")
    (message `/Game/Blueprints/Interfaces/BP_Shift.Shift` _hitactor)))

(event `SlowTime`
  ;[1 1 1] Slow Time
  (bind _output_get (set `self.TimeSlowAmount` 0.3))
  (`GameplayStatics.SetGlobalTimeDilation` _output_get)
  (set `self.CustomTimeDilation` (/ 1.0 (`self.TimeSlowAmount`)))
  (`KismetSystemLibrary.Delay` 3.0)
  (`GameplayStatics.SetGlobalTimeDilation` 1.0)
  (set `self.CustomTimeDilation` 1.0))

(event `PickupItem`
  (bind _camera (`self.Camera`))
  (bind _grabbedobject (`self.GrabbedObject`))
  (bind _returnvalue (`SceneComponent.K2_GetComponentLocation` _camera))
  ;[1 1 1] PickUpEvent
  (bind (_outhit _returnvalue_2) (`KismetSystemLibrary.LineTraceSingle` _returnvalue (+ _returnvalue (* (`SceneComponent.GetForwardVector` _camera) 1000.0)) "TraceTypeQuery1"))
  (if _returnvalue_2
    (bind (_bblockinghit _binitialoverlap _time _distance _location _impactpoint _normal _impactnormal _physmat _hitactor _hitcomponent) (`GameplayStatics.BreakHitResult` _outhit))
    (if (`SceneComponent.IsSimulatingPhysics` _hitcomponent "None")
      (bind _output_get (set `self.GrabbedObject` _hitcomponent))
      (`PhysicsHandleComponent.GrabComponentAtLocationWithRotation` (`self.PhysicsHandle`) _output_get "None" (`SceneComponent.K2_GetComponentLocation` _grabbedobject) (`SceneComponent.K2_GetComponentRotation` _grabbedobject))
      (set `self.isHoldingObject?` true))))

(event `DropObject`
  ;[1 1 1] DropObjectEvent
  (`PhysicsHandleComponent.ReleaseComponent` (`self.PhysicsHandle`))
  (set `self.isHoldingObject?` false))

(event `InputAction|Interact`
  (params (Key :type "Key Structure"))
  (:`Pressed`
    (`|SpawnActorFromClass` "/Game/Blueprints/Props/BP_Bullet.BP_Bullet_C" (`SceneComponent.K2_GetComponentToWorld` (`self.BulletSpawnPoint`)) "Undefined" "OverrideRootScale" null null)))

(fn `UserConstructionScript`)