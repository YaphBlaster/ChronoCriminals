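; BP_PushedCube is a physics prop whose AddForceToCube event applies a velocity-based acceleration to its Cube component.
; The force follows horizontal velocity and opposes vertical velocity at a hundredfold strength, ignoring mass.
; A SlowDown timeline that would print velocity and repeat this force, and a large forward push, are both disconnected.
; BeginPlay, Tick and the construction script are empty, and nothing in this Blueprint's live graph calls the event.
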(event `self.ReceiveBeginPlay`)

(event `self.ReceiveTick`
  (params (DeltaSeconds :type "Float (single-precision)")))

(event `AddForceToCube`
  (`PrimitiveComponent.AddForce` (`self.Cube`) (* (* (`SceneComponent.GetComponentVelocity` (`self.Cube`)) -1) (-1.0 -1.0 100.0)) "None" true))

(fn `UserConstructionScript`)