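; BP_Button is an interactable prop that lets a player slow time while standing inside its Trigger volume.
; Trigger overlap casts to BP_Player and BP_PlayerController, enabling the button's input on entry and disabling it on exit.
; While input is enabled, pressing Interact calls SlowTime on the player captured by the begin-overlap cast.
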(event `self.Trigger.OnComponentBeginOverlap`
  (params (OverlappedComponent :type "PrimitiveComponent Object Reference") (OtherActor :type "Actor Object Reference") (OtherComp :type "PrimitiveComponent Object Reference") (OtherBodyIndex :type Integer) (bFromSweep :type Boolean) (SweepResult :type "HitResult Structure (by ref)"))
  (bind _asbp_player (cast `/Game/Blueprints/Characters/BP_Player` OtherActor))
  (bind _asbp_player_controller (cast `/Game/Blueprints/Characters/BP_PlayerController` (`Pawn.GetController` _asbp_player)))
  (`self.EnableInput` _asbp_player_controller))

(event `InputAction|Interact`
  (params (Key :type "Key Structure"))
  (:`Pressed`
    (`/Game/Blueprints/Characters/BP_Player.SlowTime` (stale `self.Trigger.OnComponentBeginOverlap` _asbp_player))))

(event `self.Trigger.OnComponentEndOverlap`
  (params (OverlappedComponent :type "PrimitiveComponent Object Reference") (OtherActor :type "Actor Object Reference") (OtherComp :type "PrimitiveComponent Object Reference") (OtherBodyIndex :type Integer))
  (bind _asbp_player (cast `/Game/Blueprints/Characters/BP_Player` OtherActor))
  (bind _asbp_player_controller (cast `/Game/Blueprints/Characters/BP_PlayerController` (`Pawn.GetController` _asbp_player)))
  (`self.DisableInput` _asbp_player_controller))

(fn `UserConstructionScript`)