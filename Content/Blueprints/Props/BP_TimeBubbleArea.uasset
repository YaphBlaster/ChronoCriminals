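; BP_TimeBubbleArea is a prop volume that slows the player and physics objects inside it.
; On overlap begin, TimeTriggerArea sets a low CustomTimeDilation on actors whose overlapping component simulates physics, or on BP_Player.
; On overlap end, the player's dilation returns to normal.
; Physics components instead get damping set from "Original" variables the graph never assigns, leaving their actor's dilation unreset.
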(event `self.TimeTriggerArea.OnComponentBeginOverlap`
  (params (OverlappedComponent :type "PrimitiveComponent Object Reference") (OtherActor :type "Actor Object Reference") (OtherComp :type "PrimitiveComponent Object Reference") (OtherBodyIndex :type Integer) (bFromSweep :type Boolean) (SweepResult :type "HitResult Structure (by ref)"))
  ;[1 1 1] TriggerEnter
  (if (`SceneComponent.IsSimulatingPhysics` OtherComp "None")
    (set `Actor.CustomTimeDilation` 0.1 OtherActor)
    (else
      (bind _asbp_player (cast `/Game/Blueprints/Characters/BP_Player` OtherActor))
      (set `Actor.CustomTimeDilation` 0.1 _asbp_player))))

(event `self.TimeTriggerArea.OnComponentEndOverlap`
  (params (OverlappedComponent :type "PrimitiveComponent Object Reference") (OtherActor :type "Actor Object Reference") (OtherComp :type "PrimitiveComponent Object Reference") (OtherBodyIndex :type Integer))
  ;[1 1 1] TriggerExit
  (if (`SceneComponent.IsSimulatingPhysics` OtherComp "None")
    (`PrimitiveComponent.SetAngularDamping` OtherComp (`self.OriginalAngularDampening`))
    (`PrimitiveComponent.SetLinearDamping` OtherComp (`self.OriginalLinearDampening`))
    (else
      (bind _asbp_player (cast `/Game/Blueprints/Characters/BP_Player` OtherActor))
      (set `Actor.CustomTimeDilation` 1.0 _asbp_player))))

(fn `UserConstructionScript`)